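; BP_Door is a double sliding door that toggles between closed and open on each InteractDoor call.
; At BeginPlay it optionally teleports to TargetPlacementOrigin, caches both leaf positions, and triggers the toggle immediately if IsOpen is set.
; A FlipFlop alternately plays and reverses two timelines, which lerp each leaf toward its Arrow component with sweep.
; IsOpen is inverted only on the play branch.
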(event `self.ReceiveBeginPlay`
  (`|ExecutionSequence`
    (:`then_0`
      (if (`self.IsMove`)
        (`SceneComponent.K2_SetWorldLocation` (`self.DefaultSceneRoot`) (`self.K2_GetActorLocation` (`self.TargetPlacementOrigin`)) false true)))
    (:`then_1`
      (set `self.originDoorRight` (`SceneComponent.K2_GetComponentLocation` (`self.DoorRigth`)))
      (set `self.originDoorLeft` (`SceneComponent.K2_GetComponentLocation` (`self.DoorLeft`))))
    (:`then_2`
      (if (`self.IsOpen`)
        (`/Engine/EditorBlueprintResources/StandardMacros.FlipFlop` :!label _label
          (:`A`
            (`|ExecutionSequence`
              (:`then_0`
                (set `self.IsOpen` (not (`self.IsOpen`)))
                (bind (_direction _newtrack_2) (`Timeline|Timeline_2` :!label _label_2)
                  (:`Update`
                    (`SceneComponent.K2_SetWorldLocation` (`self.DoorLeft`) (`KismetMathLibrary.VLerp` (`self.originDoorLeft`) (`SceneComponent.K2_GetComponentLocation` (`self.Arrow`)) _newtrack_2) true false))))
              (:`then_1`
                (bind (_direction_2 _newtrack_2_2) (`Timeline|Timeline_1` :!label _label_3)
                  (:`Update`
                    (`SceneComponent.K2_SetWorldLocation` (`self.DoorRigth`) (`KismetMathLibrary.VLerp` (`self.originDoorRight`) (`SceneComponent.K2_GetComponentLocation` (`self.Arrow1`)) _newtrack_2_2) true false))))))
          (:`B`
            (`|ExecutionSequence`
              (:`then_0`
                (goto _label_2 :!via `Reverse`))
              (:`then_1`
                (goto _label_3 :!via `Reverse`)))))))))

(event `InteractDoor`
  (goto _label))

(fn `UserConstructionScript`)