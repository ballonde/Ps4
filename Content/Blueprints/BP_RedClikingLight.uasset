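; A red warning point light that blinks until its linked door opens, then turns solid green.
; BeginPlay plays the ClikingLight timeline, which drives the light intensity each update.
; Tick polls the target door's IsOpen and, while true, calls ForgeOn every frame to set IsOn, switch color to green, fix intensity and stop the timeline.
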(event `self.ReceiveBeginPlay`
  (bind (_direction _lightintensity) (`Timeline|ClikingLight` :!label _label)
    (:`Update`
      (`LightComponent.SetIntensity` (`self.PointLight`) _lightintensity))))

(event `ForgeOn`
  (bind _pointlight (`self.PointLight`))
  (set `self.isOn` true)
  (`LightComponent.SetLightColor` _pointlight (struct :`R` 0.14662 :`G` 1.0 :`A` 1.0) true)
  (`LightComponent.SetIntensity` _pointlight 20000.0)
  (goto _label :!via `Stop`))

(event `self.ReceiveTick`
  (params (DeltaSeconds :type "Float (single-precision)"))
  (if (`/Game/Blueprints/BP_Door.IsOpen` (`self.BP_Target_Door`))
    (`self.ForgeOn`)))

(fn `UserConstructionScript`)