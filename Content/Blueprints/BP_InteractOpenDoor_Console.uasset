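; Interactable console, going by its name a door opener, that animates a lever when used.
; Interact runs the parent class's logic, then calls LeverAnimation, which plays a timeline to rotate the Lever component with sweep enabled.
; Each update lerps from the lever's current rotation, rather than a stored start, toward the NewRotation variable, so the timeline alpha compounds.
; Any door-opening logic lies outside this file.
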(event `LeverAnimation`
  (bind (_direction _newtrack_0) (`Timeline|Timeline_0`)
    (:`Update`
      (`SceneComponent.K2_SetRelativeRotation` (`self.Lever`) (`KismetMathLibrary.RLerp` (`SceneComponent.RelativeRotation` (`self.Lever`)) (`self.New Rotation`) _newtrack_0) true false))))

(fn `Interact`
  (`parent.Interact`)
  (`self.LeverAnimation`))

(fn `UserConstructionScript`
  (`parent.UserConstructionScript`))