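; BP_C_FollowerEnnemy is an AI enemy that kills the player on contact.
; On BeginPlay its AI controller runs the follower behavior tree and stores the player pawn in the blackboard.
; When its box overlaps the first-person character, it sets the player controller's respawn point, reboots if blacked out, plays the dying sequence and calls Death.
; A disconnected, near-duplicate death chain remains in the graph.
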(event `self.ReceiveBeginPlay`
  (bind _asaicontroller (cast `AIController` (`self.GetController`)))
  (`AIController.RunBehaviorTree` _asaicontroller "/Game/AI/BT_FollowersEn.BT_FollowersEn")
  (bind _blackboardcomponent (`AIController.UseBlackboard` _asaicontroller "/Game/AI/BB_FollowerEn.BB_FollowerEn"))
  (bind _output_get (set `self.BlackboardComponent` _blackboardcomponent))
  (`BlackboardComponent.SetValueAsObject` _output_get "Player" (`GameplayStatics.GetPlayerPawn` 0)))

(event `self.Box.OnComponentBeginOverlap`
  (params (OverlappedComponent :type "PrimitiveComponent Object Reference") (OtherActor :type "Actor Object Reference") (OtherComp :type "PrimitiveComponent Object Reference") (OtherBodyIndex :type Integer) (bFromSweep :type Boolean) (SweepResult :type "HitResult Structure (by ref)"))
  (cast `/Game/Blueprints/BP_FirstPersonCharacter` OtherActor)
  (bind _asbp_playercontroller (cast `/Game/Blueprints/BP_Playercontroller` (`GameplayStatics.GetPlayerController` 0)))
  (set `/Game/Blueprints/BP_Playercontroller.LastRespawnPoint` (`self.RespawnSet`) _asbp_playercontroller)
  (if (`/Game/Blueprints/BP_Playercontroller.IsBlackOut` _asbp_playercontroller)
    (`/Game/Blueprints/BP_Playercontroller.Reboot` _asbp_playercontroller))
  (bind (_outactor _returnvalue) (`LevelSequencePlayer.CreateLevelSequencePlayer` "/Game/Cinematic/LS_Dying.LS_Dying"))
  (`MovieSceneSequencePlayer.Play` _returnvalue)
  (`/Game/Blueprints/BP_Playercontroller.Death` _asbp_playercontroller))

(fn `UserConstructionScript`)