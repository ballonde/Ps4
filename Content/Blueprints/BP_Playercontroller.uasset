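; Player controller that runs the game flow: start menu, intro sequence, UI widgets, messages, interaction and death respawn at the last respawn point.
; It also owns the player's energy, where draining to zero triggers a blackout that freezes the character for a randomly placed click QTE.
; Each reboot lowers maximum energy down to a floor and can lengthen the next QTE.
; A looping delayed event pulses a glitch overlay when maximum energy is low.
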(event `self.ReceiveBeginPlay`
  (bind _returnvalue (`|CreateWidget` "/Game/UI/WBP_Menu.WBP_Menu_C"))
  (bind _output_get (set `self.UIMenu` _returnvalue))
  (`UserWidget.AddToViewport` _output_get 0)
  (bind _asfirst_person_character (cast `/Game/Blueprints/BP_FirstPersonCharacter` (`GameplayStatics.GetPlayerPawn` 0)))
  (set `/Game/Blueprints/BP_FirstPersonCharacter.IsImmo` true _asfirst_person_character)
  (set `self.bShowMouseCursor` true))

(event `StartGame`
  (bind (_outactor _returnvalue) (`LevelSequencePlayer.CreateLevelSequencePlayer` "/Game/Cinematic/LS_Beginning.LS_Beginning"))
  (`MovieSceneSequencePlayer.Play` _returnvalue)
  (`Widget.RemoveFromParent` (`self.UIMenu`))
  (bind _asfirst_person_character (cast `/Game/Blueprints/BP_FirstPersonCharacter` (`GameplayStatics.GetPlayerPawn` 0)))
  (set `/Game/Blueprints/BP_FirstPersonCharacter.IsImmo` false _asfirst_person_character)
  (set `self.bShowMouseCursor` false)
  (bind _returnvalue_2 (`|CreateWidget` "/Game/UI/WBP_Energie.WBP_Energie_C"))
  (bind _output_get (set `self.UIEnergy` _returnvalue_2))
  (`self.ResetEnergyMaxCurrent`)
  (`self.ResetEnergy`)
  (`UserWidget.AddToViewport` _output_get 0)
  (bind _returnvalue_3 (`|CreateWidget` "/Game/UI/WBP_Message.WBP_Message_C"))
  (bind _output_get_2 (set `self.UIMessage` _returnvalue_3))
  (`UserWidget.AddToViewport` _output_get_2 0)
  (`Widget.SetVisibility` (`/Game/UI/WBP_Message.CanvasPanel_1` (`self.UIMessage`)) "Hidden")
  (`Widget.SetVisibility` (`/Game/UI/WBP_Message.PanelChoice` (`self.UIMessage`)) "Hidden")
  (`MediaPlayer.OpenSource` (`self.MediaBorderEnergy`) "/Game/Movies/Border.Border")
  (`MediaPlayer.OpenSource` (`self.MediaBackgroundBarEnergy`) "/Game/Movies/EnergyBackground.EnergyBackground")
  (`MediaPlayer.OpenSource` (`self.MediaBarEnergy`) "/Game/Movies/EnergyBar.EnergyBar")
  (`MediaPlayer.OpenSource` (`self.MediaGlitch`) "/Game/Movies/Glitch_MP4.Glitch_MP4")
  (add `self.DeathPlayer` (delegate `ResetPlayer`))
  (`Image.SetOpacity` (`/Game/UI/WBP_Energie.Glitch` (`self.UIEnergy`)) 0.0)
  (`self.GlitchDisplay`)
  (bind _returnvalue_4 (`|CreateWidget` "/Game/UI/WBP_Controls.WBP_Controls_C"))
  (bind _output_get_3 (set `self.UIControls` _returnvalue_4))
  (`UserWidget.AddToViewport` _output_get_3 0))

(event `Death`
  ;[1 1 1] DeathPlayer
  (`self.DeathPlayer`))

(event `ResetPlayer`
  ;[1 1 1] DeathPlayer
  (if (`self.IsBlackOut`)
    (`self.Reboot`))
  (bind _asfirst_person_character (cast `/Game/Blueprints/BP_FirstPersonCharacter` (`GameplayStatics.GetPlayerPawn` 0)))
  (`self.K2_SetActorLocation` _asfirst_person_character (`self.K2_GetActorLocation` (`self.LastRespawnPoint`)) false false)
  (`SceneComponent.K2_SetWorldRotation` (`/Game/Blueprints/BP_FirstPersonCharacter.FirstPersonCamera` _asfirst_person_character) (`SceneComponent.K2_GetComponentRotation` (`/Game/Blueprints/BP_RespawnPoint.Arrow` (`self.LastRespawnPoint`))) false false)
  (`self.ResetEnergyMaxCurrent`)
  (`self.ResetEnergy`))

(event `BlackOut`
  ;[1 1 1] Reboot
  (`MediaPlayer.OpenSource` (`self.MediaBlackOut`) "/Game/Movies/Reboot_MP4.Reboot_MP4")
  (`MediaPlayer.OpenSource` (`self.MediaPLayerQTE`) "/Game/Movies/QTE_Power.QTE_Power")
  (bind _returnvalue (`|CreateWidget` "/Game/UI/WBP_BlackOut.WBP_BlackOut_C"))
  (bind _output_get (set `self.UIBlackOut` _returnvalue))
  (`UserWidget.AddToViewport` _output_get 0)
  (bind _asfirst_person_character (cast `/Game/Blueprints/BP_FirstPersonCharacter` (`GameplayStatics.GetPlayerPawn` 0)))
  (set `/Game/Blueprints/BP_FirstPersonCharacter.IsImmo` true _asfirst_person_character)
  (set `self.IsBlackOut` true)
  (set `self.IndexQte` 0)
  (set `self.bShowMouseCursor` true)
  (`self.DisplayQTEClick`))

(event `ResetEnergy`
  ;[1 1 1] Energy
  (bind _output_get (set `self.Energy` (`self.EnergyMax`)))
  (`self.UpdatEnergyMax` _output_get)
  (`/Game/UI/WBP_Energie.UpdateEnergyBar` (`self.UIEnergy`) (/ (`KismetMathLibrary.Conv_IntToDouble` (`self.Energy`)) (`KismetMathLibrary.Conv_IntToDouble` (`self.EnergyMaxInitiale`)))))

(event `ResetEnergyMaxCurrent`
  ;[1 1 1] Energy
  (set `self.EnergyMax` (`self.EnergyMaxInitiale`))
  (set `self.NbClick` 0)
  (if (<= (`self.EnergyMax`) 1200)
    (`Image.SetOpacity` (`/Game/UI/WBP_Energie.Glitch` (`self.UIEnergy`)) (- 1.25 (/ (`KismetMathLibrary.Conv_IntToDouble` (`self.EnergyMax`)) (`KismetMathLibrary.Conv_IntToDouble` (`self.EnergyMaxInitiale`)))))
    (else
      (`Image.SetOpacity` (`/Game/UI/WBP_Energie.Glitch` (`self.UIEnergy`)) 0.0))))

(event `Reboot`
  ;[1 1 1] Reboot
  (`GameplayStatics.PlaySoundAtLocation` "/Game/Sound/More/PoweringAgain.PoweringAgain" (0.0 0.0 0.0) (struct) 1.0 1.0 0.0 null null null)
  (`Widget.RemoveFromParent` (`self.UIBlackOut`))
  (set `self.IsBlackOut` false)
  (bind _asfirst_person_character (cast `/Game/Blueprints/BP_FirstPersonCharacter` (`GameplayStatics.GetPlayerPawn` 0)))
  (set `/Game/Blueprints/BP_FirstPersonCharacter.IsImmo` false _asfirst_person_character)
  (set `self.bShowMouseCursor` false)
  (set `self.EnergyMax` (- (`self.EnergyMax`) (`self.ReducEnergyReboot`)))
  (if (<= (`self.EnergyMax`) 399)
    (set `self.EnergyMax` 400)
    (else
      (set `self.NbClick` (+ (`self.NbClick`) 2))))
  (`self.UpdatEnergyMax` (`self.EnergyMax`))
  (`self.ResetEnergy`))

(event `UpdateEnergy`
  (params (B :type Integer))
  ;[1 1 1] Energy
  (if (not (`self.IsBlackOut`))
    (set `self.Energy` (`KismetMathLibrary.Clamp` (- (`self.Energy`) B) 0 (`self.EnergyMax`)))
    (`/Game/UI/WBP_Energie.UpdateEnergyBar` (`self.UIEnergy`) (/ (`KismetMathLibrary.Conv_IntToDouble` (`self.Energy`)) (`KismetMathLibrary.Conv_IntToDouble` (`self.EnergyMaxInitiale`))))
    (if (<= (`self.Energy`) 0)
      (`GameplayStatics.PlaySoundAtLocation` "/Game/Sound/More/PowerOff.PowerOff" (0.0 0.0 0.0) (struct) 1.0 1.0 0.0 null null null)
      (`self.BlackOut`))))

(event `UpdatEnergyMax`
  (params (EnergyMax :type Integer))
  ;[1 1 1] Energy
  (set `self.EnergyMax` (`KismetMathLibrary.Clamp` EnergyMax 0 (`self.EnergyMaxInitiale`)))
  (`/Game/UI/WBP_Energie.UpdateEnergyBar` (`self.UIEnergy`) 0.0)
  (`/Game/UI/WBP_Energie.EnergyBarLost` (`self.UIEnergy`) (- 1.0 (/ (`KismetMathLibrary.Conv_IntToDouble` (`self.Energy`)) (`KismetMathLibrary.Conv_IntToDouble` (`self.EnergyMaxInitiale`)))))
  (if (<= (`self.EnergyMax`) 1200)
    (`Image.SetOpacity` (`/Game/UI/WBP_Energie.Glitch` (`self.UIEnergy`)) (- 1.25 (/ (`KismetMathLibrary.Conv_IntToDouble` (`self.EnergyMax`)) (`KismetMathLibrary.Conv_IntToDouble` (`self.EnergyMaxInitiale`)))))))

(event `CheckProgressQTE`
  ;[1 1 1] Reboot
  (`GameplayStatics.PlaySoundAtLocation` "/Game/Sound/More/BipPower.BipPower" (0.0 0.0 0.0) (struct) 1.0 1.0 0.0 null null null)
  (bind _result (`/Engine/EditorBlueprintResources/StandardMacros.IncrementInt` (`self.IndexQte`))
    (:`  `
      (set `self.IndexQte` _result)
      (if (<= (`self.IndexQte`) (`self.NbClick`))
        (`self.DisplayQTEClick`)
        (else
          (set `self.bShowMouseCursor` false)
          (`self.Reboot`))))))

(event `DisplayQTEClick`
  (bind (_sizex _sizey) (`self.GetViewportSize`))
  ;[1 1 1] Reboot
  (`/Game/UI/WBP_BlackOut.DisplayAleaButton` (`self.UIBlackOut`) (`KismetMathLibrary.RandomIntegerInRange` 0 (- _sizex 500)) (`KismetMathLibrary.RandomIntegerInRange` 0 (- _sizey 500))))

(event `DisplayMessage`
  (params (InText :type Text) (InText2 :type Text))
  ;[1 1 1] DisplayMessage
  (`/Game/UI/WBP_Message.DisplayMessageUpdate` (`self.UIMessage`) InText InText2)
  (`Widget.SetVisibility` (`/Game/UI/WBP_Message.CanvasPanel_1` (`self.UIMessage`)) "Visible")
  (bind _asfirst_person_character (cast `/Game/Blueprints/BP_FirstPersonCharacter` (`GameplayStatics.GetPlayerPawn` 0)))
  (set `/Game/Blueprints/BP_FirstPersonCharacter.IsImmo` true _asfirst_person_character))

(event `DisplayChoiceYesNo`
  ;[1 1 1] DisplayMessage
  (`Widget.SetVisibility` (`/Game/UI/WBP_Message.PanelChoice` (`self.UIMessage`)) "Visible")
  (set `self.bShowMouseCursor` true)
  (bind _asfirst_person_character (cast `/Game/Blueprints/BP_FirstPersonCharacter` (`GameplayStatics.GetPlayerPawn` 0)))
  (set `/Game/Blueprints/BP_FirstPersonCharacter.IsImmo` true _asfirst_person_character))

(event `GlitchDisplay`
  ;[1 1 1] Display Effect Glich
  (if (<= (`self.EnergyMax`) 1200)
    (`Image.SetOpacity` (`/Game/UI/WBP_Energie.Glitch` (`self.UIEnergy`)) (- 1.25 (/ (`KismetMathLibrary.Conv_IntToDouble` (`self.EnergyMax`)) (`KismetMathLibrary.Conv_IntToDouble` (`self.EnergyMaxInitiale`)))))
    (`KismetSystemLibrary.Delay` 2.0)
    (else
      (`KismetSystemLibrary.Delay` 2.0)))
  (`Image.SetOpacity` (`/Game/UI/WBP_Energie.Glitch` (`self.UIEnergy`)) 0.0)
  (`self.GlitchDisplay`))

(event `StopDisplayMessage`
  ;[1 1 1] DisplayMessage
  (`Widget.SetVisibility` (`/Game/UI/WBP_Message.CanvasPanel_1` (`self.UIMessage`)) "Hidden")
  (bind _asfirst_person_character (cast `/Game/Blueprints/BP_FirstPersonCharacter` (`GameplayStatics.GetPlayerPawn` 0)))
  (set `/Game/Blueprints/BP_FirstPersonCharacter.IsImmo` false _asfirst_person_character))

(event `StopDisplayChoiceYesNo`
  ;[1 1 1] DisplayMessage
  (`Widget.SetVisibility` (`/Game/UI/WBP_Message.PanelChoice` (`self.UIMessage`)) "Hidden")
  (set `self.bShowMouseCursor` false)
  (bind _asfirst_person_character (cast `/Game/Blueprints/BP_FirstPersonCharacter` (`GameplayStatics.GetPlayerPawn` 0)))
  (set `/Game/Blueprints/BP_FirstPersonCharacter.IsImmo` false _asfirst_person_character))

(event `InputAction|Interact`
  (params (Key :type "Key Structure"))
  ;[1 1 1] DisplayMessage
  (:`Pressed`
    (if (`self.CanInteract`)
      (bind _asbp_interact_object (cast `/Game/Blueprints/BP_InteractObject` (`self.OvelappingActor`)))
      (`/Game/Blueprints/BP_InteractObject.Interact` _asbp_interact_object))))

(fn `UserConstructionScript`)