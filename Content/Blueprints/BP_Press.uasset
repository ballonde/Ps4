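; BP_Press is a moving press hazard that kills the player on contact.
; On BeginPlay a timeline drives the actor's location by lerping between the positions of two referenced target actors, without sweeping.
; When its Box component overlaps a BP_FirstPersonCharacter, it calls Death on player controller 0, cast to BP_Playercontroller.
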(event `self.ReceiveBeginPlay`
  (bind (_direction _newtrack_2) (`Timeline|Timeline_0`)
    (:`Update`
      (`self.K2_SetActorLocation` (`KismetMathLibrary.VLerp` (`self.K2_GetActorLocation` (`self.Target1`)) (`self.K2_GetActorLocation` (`self.Target2`)) _newtrack_2)))))

(event `self.Box.OnComponentBeginOverlap`
  (params (OverlappedComponent :type "PrimitiveComponent Object Reference") (OtherActor :type "Actor Object Reference") (OtherComp :type "PrimitiveComponent Object Reference") (OtherBodyIndex :type Integer) (bFromSweep :type Boolean) (SweepResult :type "HitResult Structure (by ref)"))
  (cast `/Game/Blueprints/BP_FirstPersonCharacter` OtherActor)
  (bind _asbp_playercontroller (cast `/Game/Blueprints/BP_Playercontroller` (`GameplayStatics.GetPlayerController` 0)))
  (`/Game/Blueprints/BP_Playercontroller.Death` _asbp_playercontroller))

(fn `UserConstructionScript`)