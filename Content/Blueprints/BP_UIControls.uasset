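; BP_UIControls is a trigger volume that shows and hides an indexed part of the player's UI controls display.
; When the player pawn enters or leaves its Box, it casts the player controller to BP_Playercontroller and calls SetVisibilityON or SetVisibilityOFF on UIControls.
; It passes its Index variable to select what is toggled.
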(event `self.Box.OnComponentBeginOverlap`
  (params (OverlappedComponent :type "PrimitiveComponent Object Reference") (OtherActor :type "Actor Object Reference") (OtherComp :type "PrimitiveComponent Object Reference") (OtherBodyIndex :type Integer) (bFromSweep :type Boolean) (SweepResult :type "HitResult Structure (by ref)"))
  (if (== OtherActor (`GameplayStatics.GetPlayerPawn` 0))
    (bind _asbp_playercontroller (cast `/Game/Blueprints/BP_Playercontroller` (`GameplayStatics.GetPlayerController` 0)))
    (`/Game/UI/WBP_Controls.SetVisibilityON` (`/Game/Blueprints/BP_Playercontroller.UIControls` _asbp_playercontroller) (`self.Index`))))

(event `self.Box.OnComponentEndOverlap`
  (params (OverlappedComponent :type "PrimitiveComponent Object Reference") (OtherActor :type "Actor Object Reference") (OtherComp :type "PrimitiveComponent Object Reference") (OtherBodyIndex :type Integer))
  (if (== OtherActor (`GameplayStatics.GetPlayerPawn` 0))
    (bind _asbp_playercontroller (cast `/Game/Blueprints/BP_Playercontroller` (`GameplayStatics.GetPlayerController` 0)))
    (`/Game/UI/WBP_Controls.SetVisibilityOFF` (`/Game/Blueprints/BP_Playercontroller.UIControls` _asbp_playercontroller) (`self.Index`))))

(fn `UserConstructionScript`)