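; BP_Elevator is an elevator actor that moves itself between two target actors, Target1 and Target2.
; A timeline track drives a lerp between the targets' locations, applied without sweep.
; The timeline starts on BeginPlay if IsActive is set and the player controller is a BP_Playercontroller.
; Tick also polls a linked target light and calls ActivateElevator to play the timeline while that light is on.
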(event `self.ReceiveBeginPlay`
  (cast `/Game/Blueprints/BP_Playercontroller` (`GameplayStatics.GetPlayerController` 0))
  (if (`self.isActive`)
    (bind (_direction _newtrack_2) (`Timeline|Timeline_0` :!label _label)
      (:`Update`
        (`self.K2_SetActorLocation` (`KismetMathLibrary.VLerp` (`self.K2_GetActorLocation` (`self.Target1`)) (`self.K2_GetActorLocation` (`self.Target2`)) _newtrack_2))))))

(event `ActivateElevator`
  (goto _label))

(event `self.ReceiveTick`
  (params (DeltaSeconds :type "Float (single-precision)"))
  (if (`/Game/Blueprints/BP_RedClikingLight.isOn` (`self.BP_TargetLight`))
    (`self.ActivateElevator`)))

(fn `UserConstructionScript`)