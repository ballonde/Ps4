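; BP_EnergyStockSpawner is a respawning pickup that resets the player's energy.
; When a BP_FirstPersonCharacter overlaps its Box, it calls ResetEnergyMaxCurrent and ResetEnergy on player 0's BP_Playercontroller.
; It then hides itself and disables collision, restoring both after a short fixed delay rather than spawning a new actor.
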(event `self.Box.OnComponentBeginOverlap`
  (params (OverlappedComponent :type "PrimitiveComponent Object Reference") (OtherActor :type "Actor Object Reference") (OtherComp :type "PrimitiveComponent Object Reference") (OtherBodyIndex :type Integer) (bFromSweep :type Boolean) (SweepResult :type "HitResult Structure (by ref)"))
  (cast `/Game/Blueprints/BP_FirstPersonCharacter` OtherActor)
  (bind _asbp_playercontroller (cast `/Game/Blueprints/BP_Playercontroller` (`GameplayStatics.GetPlayerController` 0)))
  (`/Game/Blueprints/BP_Playercontroller.ResetEnergyMaxCurrent` _asbp_playercontroller)
  (`/Game/Blueprints/BP_Playercontroller.ResetEnergy` _asbp_playercontroller)
  (`self.SetActorHiddenInGame` self true)
  (`self.SetActorEnableCollision` false)
  (`KismetSystemLibrary.Delay` 2.0)
  (`self.SetActorHiddenInGame` self false)
  (`self.SetActorEnableCollision` self true))

(fn `UserConstructionScript`)