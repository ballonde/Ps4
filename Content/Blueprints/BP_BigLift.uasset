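; Lift actor that rides through a chain of target actors once the first-person character enters its trigger box.
; A one-time overlap slides StaticMesh1 to an Arrow position, then a timeline lerps the whole actor between the current pair of targets.
; After each leg, ChangeTarget advances through the TargetsLift array and replays the timeline.
; When the array runs out, a third timeline slides the mesh on to Arrow1.
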(event `self.Box.OnComponentBeginOverlap`
  (params (OverlappedComponent :type "PrimitiveComponent Object Reference") (OtherActor :type "Actor Object Reference") (OtherComp :type "PrimitiveComponent Object Reference") (OtherBodyIndex :type Integer) (bFromSweep :type Boolean) (SweepResult :type "HitResult Structure (by ref)"))
  (cast `/Game/Blueprints/BP_FirstPersonCharacter` OtherActor)
  (`/Engine/EditorBlueprintResources/StandardMacros.DoOnce` false
    (:`Completed`
      (set `self.LocationOrigin` (`SceneComponent.K2_GetComponentLocation` (`self.StaticMesh1`)))
      (bind (_direction _newtrack_0) (`Timeline|Timeline_1` :!via `PlayFromStart`)
        (:`Update`
          (`SceneComponent.K2_SetWorldLocation` (`self.StaticMesh1`) (`KismetMathLibrary.VLerp` (`self.LocationOrigin`) (`SceneComponent.K2_GetComponentLocation` (`self.Arrow`)) _newtrack_0) true false))
        (:`Finished`
          (bind (_direction_2 _newtrack_0_2) (`Timeline|Timeline_0` :!label _label)
            (:`Update`
              (`self.K2_SetActorLocation` (`KismetMathLibrary.VLerp` (`self.K2_GetActorLocation` (`self.CurrentTargetLift1`)) (`self.K2_GetActorLocation` (`self.CurrentTargetLift2`)) _newtrack_0_2)))
            (:`Finished`
              (`self.ChangeTarget`))))))))

(event `ChangeTarget`
  (if (< (`self.Index`) (`KismetArrayLibrary.Array_Length` (`self.TargetsLift`)))
    (set `self.CurrentTargetLift1` (`self.CurrentTargetLift2`))
    (set `self.CurrentTargetLift2` (`|GetArrayItem` (`self.TargetsLift`) (`self.Index`)))
    (set `self.Index` (+ (`self.Index`) 1))
    (goto _label :!via `PlayFromStart`)
    (else
      (set `self.LocationOrigin` (`SceneComponent.K2_GetComponentLocation` (`self.Arrow1`)))
      (bind (_direction _newtrack_0) (`Timeline|Timeline_2`)
        (:`Update`
          (`SceneComponent.K2_SetWorldLocation` (`self.StaticMesh1`) (`KismetMathLibrary.VLerp` (`SceneComponent.K2_GetComponentLocation` (`self.Arrow`)) (`self.LocationOrigin`) _newtrack_0) true false))))))

(fn `UserConstructionScript`)