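; BP_InteractOpenDoor is an interactable trigger that opens or toggles a set of linked doors.
; Its Box overlap events register it as the player controller's overlapping actor and clear that reference on exit, though both set CanInteract to true.
; The Interact override loops through the OpenDoor array and calls InteractDoor on each BP_Door, stopping early if a cast fails.
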(event `self.Box.OnComponentBeginOverlap`
  (params (OverlappedComponent :type "PrimitiveComponent Object Reference") (OtherActor :type "Actor Object Reference") (OtherComp :type "PrimitiveComponent Object Reference") (OtherBodyIndex :type Integer) (bFromSweep :type Boolean) (SweepResult :type "HitResult Structure (by ref)"))
  (bind _asbp_playercontroller (cast `/Game/Blueprints/BP_Playercontroller` (`GameplayStatics.GetPlayerController` 0)))
  (set `/Game/Blueprints/BP_Playercontroller.CanInteract` true _asbp_playercontroller)
  (set `/Game/Blueprints/BP_Playercontroller.OvelappingActor` self _asbp_playercontroller))

(event `self.Box.OnComponentEndOverlap`
  (params (OverlappedComponent :type "PrimitiveComponent Object Reference") (OtherActor :type "Actor Object Reference") (OtherComp :type "PrimitiveComponent Object Reference") (OtherBodyIndex :type Integer))
  (bind _asbp_playercontroller (cast `/Game/Blueprints/BP_Playercontroller` (`GameplayStatics.GetPlayerController` 0)))
  (set `/Game/Blueprints/BP_Playercontroller.CanInteract` true _asbp_playercontroller)
  (set `/Game/Blueprints/BP_Playercontroller.OvelappingActor` null _asbp_playercontroller))

(fn `Interact`
  (while (< (`self.Index`) (`KismetArrayLibrary.Array_Length` (`self.OpenDoor`)))
    (bind _asbp_door (cast `/Game/Blueprints/BP_Door` (`|GetArrayItem` (`self.OpenDoor`) (`self.Index`))))
    (`/Game/Blueprints/BP_Door.InteractDoor` _asbp_door)
    (set `self.Index` (+ (`self.Index`) 1)))
  (set `self.Index` 0))

(fn `UserConstructionScript`)