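; BP_HidePlace is a hiding spot whose box overlap controls whether the player counts as hidden.
; Any begin overlap sets IsHiding on the player controller and clears the PlayerVisible blackboard key on every BP_C_SimpleEnnemy, without checking the overlapping actor.
; End overlap clears IsHiding and ends the player's crouch if a short upward visibility trace finds nothing overhead.
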(event `self.Box.OnComponentBeginOverlap`
  (params (OverlappedComponent :type "PrimitiveComponent Object Reference") (OtherActor :type "Actor Object Reference") (OtherComp :type "PrimitiveComponent Object Reference") (OtherBodyIndex :type Integer) (bFromSweep :type Boolean) (SweepResult :type "HitResult Structure (by ref)"))
  (bind _asbp_playercontroller (cast `/Game/Blueprints/BP_Playercontroller` (`GameplayStatics.GetPlayerController` 0)))
  (set `/Game/Blueprints/BP_Playercontroller.IsHiding` true _asbp_playercontroller)
  (bind _outactors (`GameplayStatics.GetAllActorsOfClass` "/Game/Blueprints/BP_C_SimpleEnnemy.BP_C_SimpleEnnemy_C"))
  (for _array_element _outactors
    (`BlackboardComponent.SetValueAsBool` (`/Game/Blueprints/BP_C_SimpleEnnemy.Blackboard Component` _array_element) "PlayerVisible" false)))

(event `self.Box.OnComponentEndOverlap`
  (params (OverlappedComponent :type "PrimitiveComponent Object Reference") (OtherActor :type "Actor Object Reference") (OtherComp :type "PrimitiveComponent Object Reference") (OtherBodyIndex :type Integer))
  (bind _returnvalue (`self.K2_GetActorLocation` (`GameplayStatics.GetPlayerPawn` 0)))
  (bind _asbp_playercontroller (cast `/Game/Blueprints/BP_Playercontroller` (`GameplayStatics.GetPlayerController` 0)))
  (set `/Game/Blueprints/BP_Playercontroller.IsHiding` false _asbp_playercontroller)
  (bind (_outhit _returnvalue_2) (`KismetSystemLibrary.LineTraceSingle` _returnvalue (+ _returnvalue (0.0 0.0 120.0)) "TraceTypeQuery1"))
  (if (not _returnvalue_2)
    (bind _asfirst_person_character (cast `/Game/Blueprints/BP_FirstPersonCharacter` (`GameplayStatics.GetPlayerPawn` 0)))
    (`/Game/Blueprints/BP_FirstPersonCharacter.EndCrouch` _asfirst_person_character)))

(fn `UserConstructionScript`)