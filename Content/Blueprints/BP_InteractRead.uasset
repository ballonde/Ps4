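; BP_InteractRead is an interactable readable that shows titled text page by page through BP_Playercontroller.
; Its box overlap registers it as the controller's overlapping actor, and leaving clears that reference but still sets CanInteract true.
; Each Interact call advances through the description array.
; Past the last page it resets, flags the read as ended, hides the message and, if DialogueEnd is set, shows a yes/no choice.
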(event `self.Box.OnComponentBeginOverlap`
  (params (OverlappedComponent :type "PrimitiveComponent Object Reference") (OtherActor :type "Actor Object Reference") (OtherComp :type "PrimitiveComponent Object Reference") (OtherBodyIndex :type Integer) (bFromSweep :type Boolean) (SweepResult :type "HitResult Structure (by ref)"))
  (bind _asbp_playercontroller (cast `/Game/Blueprints/BP_Playercontroller` (`GameplayStatics.GetPlayerController` 0)))
  (set `/Game/Blueprints/BP_Playercontroller.CanInteract` true _asbp_playercontroller)
  (set `/Game/Blueprints/BP_Playercontroller.OvelappingActor` self _asbp_playercontroller))

(event `self.Box.OnComponentEndOverlap`
  (params (OverlappedComponent :type "PrimitiveComponent Object Reference") (OtherActor :type "Actor Object Reference") (OtherComp :type "PrimitiveComponent Object Reference") (OtherBodyIndex :type Integer))
  (bind _asbp_playercontroller (cast `/Game/Blueprints/BP_Playercontroller` (`GameplayStatics.GetPlayerController` 0)))
  (set `/Game/Blueprints/BP_Playercontroller.CanInteract` true _asbp_playercontroller)
  (set `/Game/Blueprints/BP_Playercontroller.OvelappingActor` null _asbp_playercontroller))

(fn `Interact`
  (set `self.Index` (+ (`self.Index`) 1))
  (if (< (`self.Index`) (`KismetArrayLibrary.Array_Length` (`self.TextDescription`)))
    (bind _asbp_playercontroller (cast `/Game/Blueprints/BP_Playercontroller` (`GameplayStatics.GetPlayerController` 0)))
    (`/Game/Blueprints/BP_Playercontroller.DisplayMessage` _asbp_playercontroller (`self.TextTiltle`) (`|GetArrayItem` (`self.TextDescription`) (`self.Index`)))
    (else
      (set `self.Index` -1)
      (set `self.EndRead` true)
      (bind _asbp_playercontroller_2 (cast `/Game/Blueprints/BP_Playercontroller` (`GameplayStatics.GetPlayerController` 0)))
      (`/Game/Blueprints/BP_Playercontroller.StopDisplayMessage` _asbp_playercontroller_2)
      (if (`self.DialogueEnd`)
        (bind _asbp_playercontroller_3 (cast `/Game/Blueprints/BP_Playercontroller` (`GameplayStatics.GetPlayerController` 0)))
        (`/Game/Blueprints/BP_Playercontroller.DisplayChoiceYesNo` _asbp_playercontroller_3)))))

(fn `UserConstructionScript`)