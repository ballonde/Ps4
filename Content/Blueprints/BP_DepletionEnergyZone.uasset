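; Trigger zone that starts draining the player's energy when the first-person character enters its box.
; The first overlap, gated by a DoOnce that is never reset, starts a self-calling Depletion event that applies a set amount through the player controller's UpdateEnergy after each delay.
; The loop stops once Energy reaches zero or below; leaving the box does not stop it.
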(event `Depletion`
  (bind _asbp_playercontroller (cast `/Game/Blueprints/BP_Playercontroller` (`GameplayStatics.GetPlayerController` 0)))
  (`/Game/Blueprints/BP_Playercontroller.UpdateEnergy` _asbp_playercontroller (`self.DepletinQuentity`))
  (`KismetSystemLibrary.Delay` (`self.SpeedDepletion`))
  (if (`self.energyDepletion`)
    (bind _asbp_playercontroller_2 (cast `/Game/Blueprints/BP_Playercontroller` (`GameplayStatics.GetPlayerController` 0)))
    (if (<= (`/Game/Blueprints/BP_Playercontroller.Energy` _asbp_playercontroller_2) 0)
      (set `self.energyDepletion` false)
      (else
        (`self.Depletion`)))))

(event `self.Box.OnComponentBeginOverlap`
  (params (OverlappedComponent :type "PrimitiveComponent Object Reference") (OtherActor :type "Actor Object Reference") (OtherComp :type "PrimitiveComponent Object Reference") (OtherBodyIndex :type Integer) (bFromSweep :type Boolean) (SweepResult :type "HitResult Structure (by ref)"))
  (cast `/Game/Blueprints/BP_FirstPersonCharacter` OtherActor)
  (`/Engine/EditorBlueprintResources/StandardMacros.DoOnce` false
    (:`Completed`
      (set `self.energyDepletion` true)
      (`self.Depletion`))))

(fn `UserConstructionScript`)