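; BP_ZoneTriggerEnemy is a trigger zone that activates a list of enemies when the player enters it.
; On the first overlap of its Box by BP_FirstPersonCharacter, guarded by a DoOnce, it calls TriggerEnnemy.
; That event loops through ListEnnemy and sets each enemy's IsActiv Blackboard key to true, leaving the resulting behavior to their AI.
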(event `TriggerEnnemy`
  (while (< (`self.index`) (`KismetArrayLibrary.Array_Length` (`self.ListEnnemy`)))
    (`BlackboardComponent.SetValueAsBool` (`/Game/Blueprints/BP_C_SimpleEnnemy.Blackboard Component` (`|GetArrayItem` (`self.ListEnnemy`) (`self.index`))) "IsActiv" true)
    (`/Engine/EditorBlueprintResources/StandardMacros.IncrementInt` (`self.index`))))

(event `self.Box.OnComponentBeginOverlap`
  (params (OverlappedComponent :type "PrimitiveComponent Object Reference") (OtherActor :type "Actor Object Reference") (OtherComp :type "PrimitiveComponent Object Reference") (OtherBodyIndex :type Integer) (bFromSweep :type Boolean) (SweepResult :type "HitResult Structure (by ref)"))
  (cast `/Game/Blueprints/BP_FirstPersonCharacter` OtherActor)
  (`/Engine/EditorBlueprintResources/StandardMacros.DoOnce` false
    (:`Completed`
      (set `self.index` 0)
      (`self.TriggerEnnemy`))))

(fn `UserConstructionScript`)