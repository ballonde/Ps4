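; Simple enemy AI character that runs a behavior tree, as walker or stationary tower, and kills the player on overlap.
; BeginPlay seeds the blackboard with targets and state flags.
; PawnSensing spots a non-hiding player, switching to run speed and triggering a distance-limited line trace that reddens the spotlight or calls LostPlayer to revert.
; Footstep sounds loop by delayed recursion while moving; several older trace-based detection chains are left disconnected.
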(event `self.ReceiveBeginPlay`
  (bind _asaicontroller (cast `AIController` (`self.GetController`)))
  (`AIController.RunBehaviorTree` _asaicontroller "/Game/AI/BT_SimpleEnnemy.BT_SimpleEnnemy")
  (bind _blackboardcomponent (`AIController.UseBlackboard` _asaicontroller "/Game/AI/BB_SimpleEnnemy.BB_SimpleEnnemy"))
  (bind _output_get (set `self.Blackboard Component` _blackboardcomponent))
  (`BlackboardComponent.SetValueAsObject` _output_get "TargetCurrent" (`|GetArrayItem` (`self.TargetList`)))
  (`BlackboardComponent.SetValueAsObject` (`self.Blackboard Component`) "Player" (`GameplayStatics.GetPlayerPawn` 0))
  (set `CharacterMovementComponent.MaxWalkSpeed` (`self.WalkSpeed`) (`self.CharacterMovement`))
  (`BlackboardComponent.SetValueAsBool` (`self.Blackboard Component`) "PawnImmo" (`self.PawnTower`))
  (`BlackboardComponent.SetValueAsBool` (`self.Blackboard Component`) "IsActiv" (`self.IsActiv`))
  (`BlackboardComponent.SetValueAsRotator` (`self.Blackboard Component`) "RotatorOrigin" (`self.K2_GetActorRotation` self))
  (`self.SoundWalk`)
  (`BlackboardComponent.SetValueAsBool` (`self.Blackboard Component`) "IsTurning" (`self.IsTurn`))
  (`BlackboardComponent.SetValueAsBool` (`self.Blackboard Component`) "ShouldTurn" true)
  (if (`self.PawnTower`)
    (bind _returnvalue (`|SpawnActorFromClass` "/Script/Engine.TargetPoint" (`self.GetTransform` self) "AlwaysSpawn" "OverrideRootScale" null null))
    (`BlackboardComponent.SetValueAsObject` (`self.Blackboard Component`) "TargetCurrent" _returnvalue)))

(event `self.PawnSensing.OnSeePawn`
  (params (Pawn :type "Pawn Object Reference"))
  (cast `/Game/FirstPersonBP/Blueprints/FirstPersonCharacter` Pawn)
  (bind _asbp_playercontroller (cast `/Game/FirstPersonBP/Blueprints/BP_Playercontroller` (`GameplayStatics.GetPlayerController` 0)))
  (if (not (`/Game/FirstPersonBP/Blueprints/BP_Playercontroller.IsHiding` _asbp_playercontroller))
    (`BlackboardComponent.SetValueAsBool` (`self.Blackboard Component`) "PlayerVisible" true)
    (set `CharacterMovementComponent.MaxWalkSpeed` (`self.RunSpeed`) (`self.CharacterMovement`))
    (set `self.TestPlayer` true)
    (bind _asabc_ennemi_simple (cast `/Game/FirstPersonBP/RobotEnnemy/Animation/ABC_EnnemiSimple` (`SkeletalMeshComponent.GetAnimInstance` (`self.Mesh`))))
    (set `/Game/FirstPersonBP/RobotEnnemy/Animation/ABC_EnnemiSimple.IsRunning` true _asabc_ennemi_simple)
    (`self.checkSigth`)))

(event `SoundWalk`
  (if (== (`self.GetVelocity` self) (0.0 0.0 0.0))
    _
    (elif (`self.TestPlayer`)
      (`GameplayStatics.PlaySoundAtLocation` "/Game/FirstPersonBP/Sound/More/BigWalk3_Cue.BigWalk3_Cue" (`self.K2_GetActorLocation` self) (struct) 1.0 1.0 0.0 null null null)
      (`KismetSystemLibrary.Delay` 0.25)
      (`self.SoundWalk`)
      (else
        (`GameplayStatics.PlaySoundAtLocation` "/Game/FirstPersonBP/Sound/More/BigWalk3_Cue.BigWalk3_Cue" (`self.K2_GetActorLocation` self) (struct) 1.0 1.0 0.0 null null null)
        (`KismetSystemLibrary.Delay` 0.4)
        (`self.SoundWalk`)))))

(event `checkSigth`
  (`KismetSystemLibrary.PrintString` "vu")
  (if (`self.TestPlayer`)
    (bind _asfirst_person_character (cast `/Game/FirstPersonBP/Blueprints/FirstPersonCharacter` (`GameplayStatics.GetPlayerPawn` 0)))
    (bind (_outhit _returnvalue) (`KismetSystemLibrary.LineTraceSingle` :`Start` (`self.K2_GetActorLocation` self) :`End` (`self.K2_GetActorLocation` _asfirst_person_character) :`TraceChannel` "TraceTypeQuery4" :`DrawDebugType` "ForDuration" :`DrawTime` 1.0))
    (if _returnvalue
      (bind (_bblockinghit _binitialoverlap _time _distance _location _impactpoint _normal _impactnormal _physmat _hitactor) (`GameplayStatics.BreakHitResult` _outhit))
      (if (<= _distance (`self.DistanceSight`))
        (cast `/Game/FirstPersonBP/Blueprints/FirstPersonCharacter` _hitactor
          (:`then`
            (`/Engine/EditorBlueprintResources/StandardMacros.DoOnce` false :!label _label
              (:`Completed`
                (`LightComponent.SetLightColor` (`self.SpotLight`) (struct :`R` 1.0 :`G` 0.01492 :`A` 1.0) true)
                (`GameplayStatics.PlaySoundAtLocation` "/Game/Interface_And_Item_Sounds/WAV/Cartoon_Falling_05.Cartoon_Falling_05" (0.0 0.0 0.0) (struct) 1.0 1.0 0.0 null null null)
                (`KismetSystemLibrary.Delay` 3.0)
                (`self.checkSigth`))))
          (:`CastFailed`
            (set `self.TestPlayer` false :!label _label_2)
            (`self.LostPlayer`)))
        (else
          (`KismetSystemLibrary.PrintString` (`KismetStringLibrary.Conv_DoubleToString` _distance))
          (goto _label_2))))))

(event `LostPlayer`
  (`LightComponent.SetLightColor` (`self.SpotLight`) (struct :`R` 1.0 :`G` 1.0 :`B` 1.0 :`A` 1.0) true)
  (cast `/Game/FirstPersonBP/Blueprints/FirstPersonCharacter` (`GameplayStatics.GetPlayerPawn` 0))
  (set `CharacterMovementComponent.MaxWalkSpeed` (`self.WalkSpeed`) (`self.CharacterMovement`))
  (`BlackboardComponent.SetValueAsBool` (`self.Blackboard Component`) "PlayerVisible" false)
  (bind _asabc_ennemi_simple (cast `/Game/FirstPersonBP/RobotEnnemy/Animation/ABC_EnnemiSimple` (`SkeletalMeshComponent.GetAnimInstance` (`self.Mesh`))))
  (set `/Game/FirstPersonBP/RobotEnnemy/Animation/ABC_EnnemiSimple.IsRunning` false _asabc_ennemi_simple)
  (set `self.TestPlayer` false)
  (goto _label :!via `Reset`))

(event `self.r.OnComponentBeginOverlap`
  (params (OverlappedComponent :type "PrimitiveComponent Object Reference") (OtherActor :type "Actor Object Reference") (OtherComp :type "PrimitiveComponent Object Reference") (OtherBodyIndex :type Integer) (bFromSweep :type Boolean) (SweepResult :type "HitResult Structure (by ref)"))
  (cast `/Game/FirstPersonBP/Blueprints/FirstPersonCharacter` OtherActor)
  (bind _asbp_playercontroller (cast `/Game/FirstPersonBP/Blueprints/BP_Playercontroller` (`GameplayStatics.GetPlayerController` 0)))
  (if (`/Game/FirstPersonBP/Blueprints/BP_Playercontroller.IsBlackOut` _asbp_playercontroller)
    (`/Game/FirstPersonBP/Blueprints/BP_Playercontroller.Reboot` _asbp_playercontroller))
  (`/Game/FirstPersonBP/Blueprints/BP_Playercontroller.Death` _asbp_playercontroller))

(fn `UserConstructionScript`)